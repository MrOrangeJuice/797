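; Elevator and lever actor that animates a rising platform and a rotating lever from two independent overlap triggers.
; Box plays the Elevator timeline to raise SMElevator along Z by a track value scaled by Lift, reversing on exit.
; Box2 likewise drives LeverTM to roll the Lever by Rotation, without affecting the elevator.
; Both set relative transforms with hardcoded locations, and neither trigger filters the overlapping actor.
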(event OnComponentBeginOverlap(Box)
  (params (OverlappedComponent :type Primitive%20Component%20Object%20Reference) (OtherActor :type Actor%20Object%20Reference) (OtherComp :type Primitive%20Component%20Object%20Reference) (OtherBodyIndex :type Integer) (bFromSweep :type Boolean) (SweepResult :type Hit%20Result%20Structure%20%28by%20ref%29))
  (bind _elevatortrack (Timeline|Elevator Play)
    (:Update
      (Transformation|ResetRelativeTransform (Variables|Default|GetSM_Elevator))
      (Transformation|SetRelativeTransform (Variables|Default|GetSM_Elevator) (Math|Transform|MakeTransform (Math|Vector|MakeVector -8e+01 0.0 (* _elevatortrack (Variables|Default|GetLift))) "0, 0, 0" "1.000000,1.000000,1.000000") false false))))

(event OnComponentEndOverlap(Box)
  (params (OverlappedComponent :type Primitive%20Component%20Object%20Reference) (OtherActor :type Actor%20Object%20Reference) (OtherComp :type Primitive%20Component%20Object%20Reference) (OtherBodyIndex :type Integer))
  (bind _elevatortrack (Timeline|Elevator Reverse)
    (:Update
      (Transformation|ResetRelativeTransform (Variables|Default|GetSM_Elevator))
      (Transformation|SetRelativeTransform (Variables|Default|GetSM_Elevator) (Math|Transform|MakeTransform (Math|Vector|MakeVector -8e+01 0.0 (* _elevatortrack (Variables|Default|GetLift))) "0, 0, 0" "1.000000,1.000000,1.000000") false false))))

(event OnComponentBeginOverlap(Box2)
  (params (OverlappedComponent :type Primitive%20Component%20Object%20Reference) (OtherActor :type Actor%20Object%20Reference) (OtherComp :type Primitive%20Component%20Object%20Reference) (OtherBodyIndex :type Integer) (bFromSweep :type Boolean) (SweepResult :type Hit%20Result%20Structure%20%28by%20ref%29))
  (bind _levertrack (Timeline|LeverTM Play)
    (:Update
      (Transformation|ResetRelativeTransform (Variables|Default|Getlever))
      (Transformation|SetRelativeTransform (Variables|Default|Getlever) (Math|Transform|MakeTransform (Math|Vector|MakeVector 0.0 -6.4e+02 0.0) (Math|Rotator|MakeRotator (* _levertrack (Variables|Default|GetRotation)) 0.0 0.0) "1.000000,1.000000,1.000000") false false))))

(event OnComponentEndOverlap(Box2)
  (params (OverlappedComponent :type Primitive%20Component%20Object%20Reference) (OtherActor :type Actor%20Object%20Reference) (OtherComp :type Primitive%20Component%20Object%20Reference) (OtherBodyIndex :type Integer))
  (bind _levertrack (Timeline|LeverTM Reverse)
    (:Update
      (Transformation|ResetRelativeTransform (Variables|Default|Getlever))
      (Transformation|SetRelativeTransform (Variables|Default|Getlever) (Math|Transform|MakeTransform (Math|Vector|MakeVector 0.0 -6.4e+02 0.0) (Math|Rotator|MakeRotator (* _levertrack (Variables|Default|GetRotation)) 0.0 0.0) "1.000000,1.000000,1.000000") false false))))

(event EventBeginPlay)

(event Collision|EventActorBeginOverlap
  (params (OtherActor :type Actor%20Object%20Reference)))

(event EventTick
  (params (DeltaSeconds :type Float%20%28single-precision%29)))

(fn ConstructionScript)