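; BP_SplinSM is a spline-driven placement actor that lays static meshes along its spline at construction time.
; Each SMData entry supplies mesh variants, spacing, an offset and a tangent flag, and the construction script adds collision-enabled spline mesh components at each interval with random variants.
; Flagged entries stretch between successive distances using spline directions; others sit at each point with spline rotation and offset.
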(event EventBeginPlay)

(event Collision|EventActorBeginOverlap
  (params (OtherActor :type Actor%20Object%20Reference)))

(event EventTick
  (params (DeltaSeconds :type Float%20%28single-precision%29)))

(fn ConstructionScript
  (bind _spline (Variables|Default|GetSpline))
  (bind _sm_data (Variables|Default|GetSM_Data))
  (bind _spline_2 (Variables|Default|GetSpline))
  (for _index (range 0 (Utilities|Array|Length _sm_data))
    (bind _output_get (Variables|Default|SetVariety (.Mesh (Utilities|Struct|BreakS_MeshData (Utilities|Array|Get(acopy) _sm_data _index)))))
    (Variables|Default|SetSpacing (.Spacing (Utilities|Struct|BreakS_MeshData (Utilities|Array|Get(acopy) _sm_data _index))))
    (Variables|Default|SetLocation (.Location (Utilities|Struct|BreakS_MeshData (Utilities|Array|Get(acopy) _sm_data _index))))
    (Variables|Default|SetTanget (.Tanget (Utilities|Struct|BreakS_MeshData (Utilities|Array|Get(acopy) _sm_data _index))))
    (for _index_2 (range 0 (+ (.ReturnValue (Math|Float|Division(WholeandRemainder) (Spline|GetSplineLength (Variables|Default|GetSpline)) (Variables|Default|GetSpacing))) (.OutIndex (Utilities|Array|Random _output_get))))
      (Variables|Default|SetDistanceA (* _index_2 (Variables|Default|GetSpacing)))
      (Variables|Default|SetDistanceB (+ (* _index_2 (Variables|Default|GetSpacing)) (Variables|Default|GetSpacing)))
      (if (Variables|Default|GetTanget)
        (bind _returnvalue (AddComponent|AddSplineMeshComponent false))
        (Components|StaticMesh|SetStaticMesh _returnvalue (.OutItem (Utilities|Array|Random _output_get)))
        (Collision|SetCollisionEnabled _returnvalue "QueryAndPhysics")
        (SplineMesh|SetStartandEnd _returnvalue (Spline|GetLocationatDistanceAlongSpline _spline_2 (Variables|Default|GetDistanceA) "Local") (Spline|GetDirectionatDistanceAlongSpline _spline_2 (Variables|Default|GetDistanceA) "Local") (Spline|GetLocationatDistanceAlongSpline _spline_2 (Variables|Default|GetDistanceB) "Local") (Spline|GetDirectionatDistanceAlongSpline _spline_2 (Variables|Default|GetDistanceB) "Local") true :!class /Script/Engine.SplineMeshComponent)
        (else
          (bind _returnvalue_2 (AddComponent|AddSplineMeshComponent false (Math|Transform|MakeTransform (+ (Spline|GetLocationatDistanceAlongSpline _spline (Variables|Default|GetDistanceA) "Local") (Variables|Default|GetLocation)) (Spline|GetRotationatDistanceAlongSpline _spline (Variables|Default|GetDistanceA) "Local"))))
          (Components|StaticMesh|SetStaticMesh _returnvalue_2 (.OutItem (Utilities|Array|Random _output_get)))
          (Collision|SetCollisionEnabled _returnvalue_2 "QueryAndPhysics"))))))